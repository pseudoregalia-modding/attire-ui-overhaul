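; Function library for the attire UI overhaul mod that swaps the active weapon skin and fits its transforms.
; ChangeActiveWeapon updates the mod actor, player and loose weapon meshes, resets their materials and saves the choice via the game instance.
; It finds the mesh's row across discovered DT_WeaponData tables, falling back to generated data.
; Row transforms offset default weapon and light transforms, and the stage weapon's height follows its bounding box.
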(fn SetWeaponSkeletalMesh
  (params (ActorComponent :type Skeletal%20Mesh%20Component%20Object%20Reference) (NewWeapon :type Skeletal%20Mesh%20Object%20Reference))
  (Components|SkeletalMesh|SetSkeletalMeshAsset ActorComponent NewWeapon)
  (for (_ _array_index) (Variables|/Script/Engine.SkeletalMesh|GetMaterials (Variables|/Script/Engine.SkeletalMeshComponent|GetSkeletalMeshAsset ActorComponent))
    (Rendering|Material|SetMaterial ActorComponent _array_index 0))
  (for (_array_element _array_index_2) (Variables|/Script/Engine.SkeletalMesh|GetMaterials NewWeapon)
    (Rendering|Material|SetMaterial ActorComponent _array_index_2 (.materialinterface _array_element)))
  (bind _gameinstance (CallFunction|GetGameInstance))
  (Utilities|SaveActiveWeapon NewWeapon _gameinstance))

(fn TransformWeaponMesh
  (params (NewTransform :type Transform) (isStage? :type Boolean))
  (if isStage?
    (bind _returnvalue (Actor|GetActorOfClass 0 "/Game/Mods/FoeHammers_AttireUIOverhaul_P/Blueprints/ModActor.ModActor_C"))
    (bind _output_get (LocalVariables|SetModWeaponMesh (Variables|/Game/Mods/FoeHammers_AttireUIOverhaul_P/Blueprints/ModActor.ModActor_C|GetWeaponMesh _returnvalue)))
    (Transformation|SetRelativeTransform _output_get (LocalVariables|GetDefaultStageWeaponTransform) false false)
    (Class|SceneComponent|AddLocalTransform _output_get NewTransform false false)
    (CallFunction|UpdateTransformBasedonBoundingBox (LocalVariables|GetModWeaponMesh)))
  (bind _returnvalue_2 (Actor|GetActorOfClass 0 "/Game/ThirdPerson/Player/BP_looseWeapon.BP_looseWeapon_C"))
  (bind _output_get_2 (LocalVariables|SetLooseWeaponMesh (Variables|/Game/ThirdPerson/Player/BP_looseWeapon.BP_looseWeapon_C|GetSkeletalMesh _returnvalue_2)))
  (Transformation|SetRelativeTransform _output_get_2 (LocalVariables|GetDefaultLooseWeaponTransform) false false)
  (Class|SceneComponent|AddLocalTransform _output_get_2 NewTransform false false))

(fn TransformLightMesh
  (params (NewTransform :type Transform))
  (bind _returnvalue (Actor|GetActorOfClass 0 "/Game/ThirdPerson/Player/BP_PlayerGoatMain.BP_PlayerGoatMain_C"))
  (Transformation|SetRelativeTransform (Variables|/Game/ThirdPerson/Player/BP_PlayerGoatMain.BP_PlayerGoatMain_C|GetLightMesh _returnvalue) (LocalVariables|GetDefaultLightTransform) false false)
  (Class|SceneComponent|AddLocalTransform (Variables|/Game/ThirdPerson/Player/BP_PlayerGoatMain.BP_PlayerGoatMain_C|GetLightMesh _returnvalue) NewTransform false false))

(fn GetActiveWeaponData
  (params (AssetData :type Array%20of%20Asset%20Data%20Structures) (ActiveWeapon :type Skeletal%20Mesh%20Object%20Reference))
  (bind _returnvalue (Utilities|GetObjectName ActiveWeapon))
  (bind (_lefts _rights _returnvalue_2) (Utilities|String|Split _returnvalue "mainWeapon_"))
  (for _array_element AssetData
    (if (and (.bSuccess (Utilities|Casting|CastToDataTable (Class|AssetRegistryHelpers|GetAsset _array_element))) (Utilities|String|Contains (Class|AssetRegistryHelpers|GetFullName _array_element) "DT_WeaponData"))
      (bind _outrownames (DataTable|GetDataTableRowNames (.AsData%20Table (Utilities|Casting|CastToDataTable (Class|AssetRegistryHelpers|GetAsset _array_element)))))
      (for _array_element_2 _outrownames
        (bind _returnvalue_3 (Utilities|GetDataTableRow (.AsData%20Table (Utilities|Casting|CastToDataTable (Class|AssetRegistryHelpers|GetAsset _array_element))) _array_element_2)
          (:then
            (if (== (Utilities|Struct|BreakST_WeaponData _returnvalue_3) ActiveWeapon)
              (LocalVariables|SetOutRow _returnvalue_3)
              (return (LocalVariables|GetOutRow))))))))
  (LocalVariables|SetOutRow (Utilities|Struct|MakeST_WeaponData (Utilities|String|StringToName (Utilities|String|SelectString (Utilities|String|Replace _rights "_" " ") "Dream Breaker" _returnvalue_2)) ActiveWeapon (Math|Transform|MakeTransform "0, 0, 0" "0, 0, 0" "1.000000,1.000000,1.000000") (Math|Transform|MakeTransform "0, 0, 0" "0, 0, 0" "0.250000,0.250000,0.400000")))
  (return (LocalVariables|GetOutRow)))

(fn GetGameInstance
  (return (.AsMV%20Game%20Instance (Utilities|Casting|CastToMV_GameInstance (Game|GetGameInstance)))))

(fn UpdateActiveWeaponMeshes
  (params (NewWeapon :type Skeletal%20Mesh%20Object%20Reference))
  (LocalVariables|SetWeaponMesh NewWeapon)
  (Utilities|FlowControl|Sequence
    (:then_0
      (bind _returnvalue (Actor|GetActorOfClass 0 "/Game/Mods/FoeHammers_AttireUIOverhaul_P/Blueprints/ModActor.ModActor_C"))
      (CallFunction|SetWeaponSkeletalMesh (Variables|/Game/Mods/FoeHammers_AttireUIOverhaul_P/Blueprints/ModActor.ModActor_C|GetWeaponMesh _returnvalue) (LocalVariables|GetWeaponMesh)))
    (:then_1
      (bind _returnvalue_2 (Actor|GetActorOfClass 0 "/Game/ThirdPerson/Player/BP_PlayerGoatMain.BP_PlayerGoatMain_C"))
      (CallFunction|SetWeaponSkeletalMesh (Variables|/Game/ThirdPerson/Player/BP_PlayerGoatMain.BP_PlayerGoatMain_C|GetWeaponMesh _returnvalue_2) (LocalVariables|GetWeaponMesh)))
    (:then_2
      (bind _returnvalue_3 (Actor|GetActorOfClass 0 "/Game/ThirdPerson/Player/BP_looseWeapon.BP_looseWeapon_C"))
      (CallFunction|SetWeaponSkeletalMesh (Variables|/Game/ThirdPerson/Player/BP_looseWeapon.BP_looseWeapon_C|GetSkeletalMesh _returnvalue_3) (LocalVariables|GetWeaponMesh)))))

(fn UpdateTransformBasedonBoundingBox
  (params (WeaponComponent :type Scene%20Component%20Object%20Reference))
  (bind _returnvalue (Transformation|GetWorldLocation WeaponComponent))
  (Transformation|SetWorldLocation WeaponComponent (Math|Vector|MakeVector (.x _returnvalue) (.y _returnvalue) (+ (.z (.BoxExtent (Collision|GetComponentBounds WeaponComponent))) (LocalVariables|GetWorld%20Z%20Offset) (LocalVariables|GetBufferOffset))) false false)
  (return))

(fn ChangeActiveWeapon
  (params (NewWeapon :type Skeletal%20Mesh%20Object%20Reference) (AssetData :type Array%20of%20Asset%20Data%20Structures) (isStage? :type Boolean))
  (CallFunction|UpdateActiveWeaponMeshes NewWeapon)
  (bind _weapondata (CallFunction|GetActiveWeaponData AssetData NewWeapon))
  (CallFunction|TransformWeaponMesh (.weapontransform _weapondata) isStage?)
  (CallFunction|TransformLightMesh (.lighttransform _weapondata)))