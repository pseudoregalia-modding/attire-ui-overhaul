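; Mod actor for an attire UI overhaul that renders a rotating preview of the player's character through a scene capture.
; On BeginPlay it limits the capture to its own components and hides the weapon unless the "attack" upgrade (Dream Breaker) is unlocked in the game instance.
; Tick spins the character mesh, and UpdatePlayerMesh copies the skeletal mesh from the given player's VisualMesh.
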(event Custom|PrintToModLoader
  (params (Message :type String)))

(event EventBeginPlay
  ;[0.4354 0.6471 1] Whitelist only Actor Components
  (Rendering|SceneCapture|ShowOnlyActorComponents (Variables|Default|GetSceneCaptureComponent2D) self true)
  ;[0 0.7422 1] Is Dream Breaker Unlocked
  (if (not (== (.Value (Utilities|Map|Find (Variables|/Game/Blueprints/GameData/MV_GameInstance.MV_GameInstance_C|GetupgradeTracker (.AsMV%20Game%20Instance (Utilities|Casting|CastToMV_GameInstance (Game|GetGameInstance)))) "attack")) 1))
    (Rendering|SetVisibility (Variables|Default|GetWeaponScene) false true)))

(event EventTick
  (params (DeltaSeconds :type Float%20%28single-precision%29))
  ;[0.1392 0.5312 0.1204] Rotate PlayerMesh
  (Transformation|AddLocalRotation (Variables|Default|GetCharacterMesh) "0.000000,0.500000,0.000000" false false))

(fn ConstructionScript)

(fn UpdatePlayerMesh
  (params (Player%20Actor :type BP%20Player%20Goat%20Main%20Object%20Reference))
  (Components|SkeletalMesh|SetSkeletalMeshAsset (Variables|ModActor_C|GetCharacterMesh self) (Components|SkeletalMesh|GetSkeletalMeshAsset (Variables|/Game/ThirdPerson/Player/BP_PlayerGoatMain.BP_PlayerGoatMain_C|GetVisualMesh Player%20Actor))))