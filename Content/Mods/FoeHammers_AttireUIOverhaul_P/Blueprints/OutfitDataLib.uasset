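; Function library for the Attire UI Overhaul mod that gathers outfit meshes and swaps the player's active outfit.
; LoadOutfitAssets loads an array of asset entries, keeping skeletal meshes that are neither main-weapon assets nor on an exclusion list.
; ChangeActiveOutfit sets the player's visual mesh, rebuilds its material list from the new mesh, resets it, then saves the choice through the MV game instance.
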(fn ChangeActiveOutfit
  (params (NewOutfit :type Skeletal%20Mesh%20Object%20Reference) (Player :type BP%20Player%20Goat%20Main%20Object%20Reference))
  (bind _meshmats (Variables|/Game/ThirdPerson/Player/BP_PlayerGoatMain.BP_PlayerGoatMain_C|GetmeshMats Player))
  (Components|SkeletalMesh|SetSkeletalMeshAsset (Variables|/Game/ThirdPerson/Player/BP_PlayerGoatMain.BP_PlayerGoatMain_C|GetVisualMesh Player) NewOutfit)
  (Utilities|Array|Clear _meshmats)
  (for _array_element (Variables|/Script/Engine.SkeletalMesh|GetMaterials NewOutfit)
    (Utilities|Array|Add _meshmats (.materialinterface _array_element)))
  (Default|MeshReset Player)
  (bind _gameinstance (CallFunction|GetGameInstance))
  (Utilities|SaveActiveOutfit NewOutfit _gameinstance))

(fn LoadOutfitAssets
  (params (Array :type Array%20of%20Asset%20Data%20Structures) (TempOutfitList :type Array%20of%20Skeletal%20Mesh%20Object%20References))
  (for _array_element Array
    (if (Math|Boolean|ANDBoolean (.bSuccess (Utilities|Casting|CastToSkeletalMesh (Class|AssetRegistryHelpers|GetAsset _array_element))) (not (Utilities|String|Contains (Class|AssetRegistryHelpers|GetFullName _array_element) "mainWeapon")) (not (Utilities|Array|ContainsItem (LocalVariables|GetexcludedAssets) (Utilities|GetObjectName (.AsSkeletal%20Mesh (Utilities|Casting|CastToSkeletalMesh (Class|AssetRegistryHelpers|GetAsset _array_element)))))))
      (Utilities|Array|Add TempOutfitList (.AsSkeletal%20Mesh (Utilities|Casting|CastToSkeletalMesh (Class|AssetRegistryHelpers|GetAsset _array_element))))))
  (return))

(fn GetGameInstance
  (return (.AsMV%20Game%20Instance (Utilities|Casting|CastToMV_GameInstance (Game|GetGameInstance)))))