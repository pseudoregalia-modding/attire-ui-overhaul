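; Function library in the FoeHammers Attire UI Overhaul mod that sets the player goat's dash afterimage colour.
; SetDashColour saves the chosen hue through SaveActiveHue with the game instance, then converts it from HSV at fixed saturation and value into the character's AfterimageColor.
; Random and default variants feed that function a random or fixed hue, and small helpers supply the cast player character and game instance.
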(fn SetDashColour
  (params (Hue :type Integer))
  (bind _asbp_player_goat_main (CallFunction|GetPlayerCharacter))
  (bind _gameinstance (CallFunction|GetGameInstance))
  (Utilities|SaveActiveHue Hue _gameinstance)
  (bind _output_get (Variables|/Game/ThirdPerson/Player/BP_PlayerGoatMain.BP_PlayerGoatMain_C|SetafterimageColor _asbp_player_goat_main (Class|KismetMathLibrary|HSVtoRGB (Math|Conversions|ToFloat(Integer) Hue) 0.737749 1.0 1.0)))
  (return _output_get))

(fn SetRandomDashColour
  (bind _outputcolour (CallFunction|SetDashColour (Math|Random|RandomInteger 360)))
  (return _outputcolour))

(fn SetDefaultColour
  (bind _outputcolour (CallFunction|SetDashColour 50))
  (return _outputcolour))

(fn GetPlayerCharacter
  (return (.AsBP%20Player%20Goat%20Main (Utilities|Casting|CastToBP_PlayerGoatMain (Game|GetPlayerCharacter 0)))))

(fn GetGameInstance
  (return (.AsMV%20Game%20Instance (Utilities|Casting|CastToMV_GameInstance (Game|GetGameInstance)))))